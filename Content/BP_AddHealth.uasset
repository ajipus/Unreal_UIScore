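; Health pickup actor that heals a BP_PlayerTask4 player on overlap with its Box component.
; If PlayerHealth is below 100, it adds 10, prints MaxHealth and destroys itself; at full health it stays.
; The cap check writes 100 to MaxHealth instead of PlayerHealth, so health can end above 100.
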(event `self.Box.OnComponentBeginOverlap`
  (params (OverlappedComponent :type "PrimitiveComponent Object Reference") (OtherActor :type "Actor Object Reference") (OtherComp :type "PrimitiveComponent Object Reference") (OtherBodyIndex :type Integer) (bFromSweep :type Boolean) (SweepResult :type "HitResult Structure (by ref)"))
  (bind _asbp_player_task_4 (cast `/Game/BP_PlayerTask4` OtherActor))
  (bind _playerhealth (`/Game/BP_PlayerTask4.PlayerHealth` _asbp_player_task_4))
  (if (< _playerhealth 100.0)
    (bind _output_get (set `/Game/BP_PlayerTask4.PlayerHealth` (+ _playerhealth 10.0) _asbp_player_task_4))
    (if (>= _output_get 100.0)
      (bind _output_get_2 (set `/Game/BP_PlayerTask4.MaxHealth` 100.0 _asbp_player_task_4))
      (else
        (set `/Game/BP_PlayerTask4.PlayerHealth` _output_get _asbp_player_task_4)))
    (`KismetSystemLibrary.PrintString` (`KismetStringLibrary.Conv_DoubleToString` _output_get_2))
    (`self.K2_DestroyActor`)))

(fn `UserConstructionScript`)